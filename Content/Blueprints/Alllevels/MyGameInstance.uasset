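; MyGameInstance is the game instance that handles the main menu, loading screen and online session hosting or joining.
; The menu event creates or reuses the MainMenu widget with UI-only input and a visible cursor.
; CreateSession shows the loading screen, creates a non-LAN session and opens LobbyMap as a listen server.
; JoinSession attempts to join every found session, then falls through into the same session-creation path.
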(event `showmainmenu`
  (bind _returnvalue (`GameplayStatics.GetPlayerController` 0))
  ;[1 1 1] Show main menu and set mouse cursor
  (`/Engine/EditorBlueprintResources/StandardMacros.IsValid` (`self.MMenuRef`)
    (:`Is Valid`
      _)
    (:`Is Not Valid`
      (bind _returnvalue_2 (`|CreateWidget` "/Game/UI/MainMenu/MainMenu.MainMenu_C"))
      (bind _output_get (set `self.MMenuRef` _returnvalue_2))))
  (`WidgetBlueprintLibrary.SetInputMode_UIOnlyEx` _returnvalue _output_get)
  (`UserWidget.AddToViewport` _output_get 0)
  (set `PlayerController.bShowMouseCursor` true _returnvalue))

(event `ShowLoadingScreen`
  ;[1 1 1] Show loading screen
  (`/Engine/EditorBlueprintResources/StandardMacros.IsValid` null
    (:`Is Valid`
      _)
    (:`Is Not Valid`
      (bind _returnvalue (`|CreateWidget` "/Game/UI/AllLevels/Loadingscreen.Loadingscreen_C" (`GameplayStatics.GetPlayerController` 0)))
      (bind _output_get (set `self.LScreenRef` _returnvalue))))
  (`UserWidget.AddToViewport` _output_get 0))

(event `CreateSession`
  ;[1 1 1] Crate Session
  (`self.ShowLoadingScreen`)
  (`CreateSessionCallbackProxy.CreateSession` (`GameplayStatics.GetPlayerController` 0) 100 :!label _label
    (:`OnSuccess`
      (`GameplayStatics.OpenLevel` "LobbyMap" true "listen"))))

(event `JoinSession`
  (bind _returnvalue (`GameplayStatics.GetPlayerController` 0))
  ;[1 1 1] Join session
  (`self.ShowLoadingScreen`)
  (bind _results (`FindSessionsCallbackProxy.FindSessions` _returnvalue 20)
    (:`OnSuccess`
      (for _array_element _results
        (`JoinSessionCallbackProxy.JoinSession` _returnvalue _array_element))
      (goto _label))))